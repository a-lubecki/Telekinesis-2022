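; Physics-driven object that can be selected, attracted, levitated and thrown through telekinesis.
; Root simulates physics, losing gravity while grabbed; Attract uses a negative radial force, and Throw applies a velocity-change impulse.
; Levitate lerps with sweep toward a destination, zeroing linear velocity and adding random spin.
; Selection outline toggles custom depth on all mesh components, whose stencil value is set at BeginPlay.
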(event EventBeginPlay
  (bind _root (Variables|Default|GetRoot))
  (Physics|SetSimulatePhysics _root true)
  (Physics|SetEnableGravity _root true)
  ;[1 1 1] Prepare outline on meshes
  (for _array_element (Actor|GetComponentsByClass "/Script/Engine.MeshComponent")
    (bind _asmesh_component (Utilities|Casting|CastToMeshComponent _array_element))
    (Rendering|SetCustomDepthStencilValue _asmesh_component 1)))

(fn ConstructionScript)

(fn SetSelectionOutlineVisible
  (params (IsOutlineVisible :type Boolean))
  ;[1 1 1] Enable outline on meshes
  (for _array_element (Actor|GetComponentsByClass "/Script/Engine.MeshComponent")
    (bind _asmesh_component (Utilities|Casting|CastToMeshComponent _array_element))
    (Rendering|SetRenderCustomDepth _asmesh_component IsOutlineVisible)))

(fn SetasGrabbed
  (params (IsGrabbed :type Boolean))
  (Physics|SetEnableGravity (Variables|Default|GetRoot) (not IsGrabbed)))

(fn Attract
  (params (Destination :type Vector))
  (Physics|AddRadialForce (Variables|Default|GetRoot) Destination 1e+05 -3e+04 "RIF_Constant" true))

(fn Levitate
  (params (Destination :type Vector))
  (bind _root (Variables|Default|GetRoot))
  (Transformation|SetWorldLocation _root (Math|Vector|Lerp(Vector) (Transformation|GetWorldLocation (Variables|Default|GetRoot)) Destination (/ (* (Utilities|Time|GetWorldDeltaSeconds) 0.5) 0.1)) true false)
  (Physics|SetPhysicsLinearVelocity _root "0, 0, 0" false "None")
  (Class|PrimitiveComponent|AddAngularImpulseinDegrees _root (Math|Vector|MakeVector (Math|Random|RandomFloatinRange -1e+01 1e+01) (Math|Random|RandomFloatinRange -1e+01 1e+01) (Math|Random|RandomFloatinRange -1e+01 1e+01)) "None" true))

(fn Throw
  (params (Orientation :type Vector))
  (Physics|AddImpulse (Variables|Default|GetRoot) (* Orientation 1e+04) "None" true))

(fn CanbeGrabbedbyPlayer
  (return (LocalVariables|GetCanBeGrabbed)))