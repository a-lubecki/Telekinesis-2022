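; BP_Enemy is an enemy that chases the player and dies when hit by a fast-moving object.
; While alive, Tick issues a move most of the way toward the player whenever they are within range.
; A high-velocity capsule hit calls SetAsDead, which disables capsule collision, removes the autolock target and ragdolls the mesh.
; It then spawns a BP_TelekinesisRagdoll and assigns the ragdolled mesh to it.
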(event OnComponentHit(CapsuleComponent)
  (params (HitComponent :type Primitive%20Component%20Object%20Reference) (OtherActor :type Actor%20Object%20Reference) (OtherComp :type Primitive%20Component%20Object%20Reference) (NormalImpulse :type Vector :default "0, 0, 0") (Hit :type Hit%20Result%20Structure%20%28by%20ref%29))
  (if (> (Math|Vector|VectorLength (Transformation|GetComponentVelocity OtherComp)) 1e+03)
    (CallFunction|SetasDead)))

(event EventTick
  (params (DeltaSeconds :type Float%20%28single-precision%29))
  (bind _returnvalue (Game|Player|GetPlayerPawn 0))
  (bind _rootcomponent (Variables|Transformation|GetRootComponent))
  (bind _returnvalue_2 (Transformation|GetWorldLocation _rootcomponent))
  (bind _rootcomponent_2 (Variables|/Script/Engine.Actor|GetRootComponent _returnvalue))
  (bind _returnvalue_3 (Transformation|GetWorldLocation _rootcomponent_2))
  ;[1 1 1] AI move
  (|CallParentFunction DeltaSeconds)
  (if (not (Variables|Default|GetIsDead))
    (if (< (Math|Vector|Distance(Vector) _returnvalue_2 _returnvalue_3) 8e+02)
      (AI|Navigation|SimpleMovetoLocation (Pawn|GetController) (Math|Vector|Lerp(Vector) _returnvalue_2 _returnvalue_3 0.8)))))

(fn ConstructionScript
  (|CallParentFunction))

(fn SetasDead
  (bind _mesh (Variables|Character|GetMesh))
  (bind _bp_autolocktarget (Variables|Default|GetBP_AutolockTarget))
  (Utilities|FlowControl|Sequence
    (:then_0
      (Variables|Default|SetIsDead true)
      (Collision|SetCollisionEnabled (Variables|Collision|GetCapsuleComponent) "NoCollision")
      (Utilities|IsValid _bp_autolocktarget
        (:Is%20Valid
          (Components|DestroyComponent _bp_autolocktarget))))
    (:then_1
      (Physics|SetSimulatePhysics _mesh true)
      (Collision|SetCollisionProfileName _mesh "Ragdoll" true :!class /Script/Engine.PrimitiveComponent)
      (Collision|SetCollisionResponsetoChannel _mesh "ECC_Pawn" "ECR_Block"))
    (:then_2
      (bind _returnvalue (Game|SpawnActorfromClass "/Game/Alubecki/Assets/Enemy/BP_TelekinesisRagdoll.BP_TelekinesisRagdoll_C" (Transformation|GetActorTransform) "Undefined" 0 0))
      (Default|AssignRagdoll _returnvalue (Variables|Character|GetMesh)))))