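; Telekinesis proxy actor that lets an assigned ragdoll skeletal mesh be grabbed, levitated, attracted and thrown.
; AssignRagdoll attaches the ragdoll's owner to this actor and prepares its outline, while Tick keeps TriggerSphere on the ragdoll.
; Grabbing disables gravity and holds the closest bone with a physics handle, which Levitate retargets while damping spine velocity.
; Attract applies negative radial force toward a destination, and Throw applies a velocity-change impulse at the spine.
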(event EventTick
  (params (DeltaSeconds :type Float%20%28single-precision%29))
  (Utilities|IsValid (Variables|Default|GetRagdoll)
    (:Is%20Valid
      (Transformation|SetWorldTransform (Variables|Default|GetTriggerSphere) (Transformation|GetWorldTransform (Variables|Default|GetRagdoll)) true false))))

(fn ConstructionScript
  (|CallParentFunction))

(fn SetasGrabbed
  (params (IsGrabbed :type Boolean))
  (bind _ragdoll (Variables|Default|GetRagdoll))
  (bind _ragdoll_2 (Variables|Default|GetRagdoll))
  (bind _returnvalue (Transformation|GetWorldLocation _ragdoll_2))
  (bind (_bonelocation _returnvalue_2) (Class|SkinnedMeshComponent|FindClosestBoneK2 _ragdoll_2 _returnvalue 0.0))
  (Utilities|IsValid _ragdoll
    (:Is%20Valid
      (Physics|SetEnableGravity _ragdoll (not IsGrabbed))
      (if IsGrabbed
        (Class|PhysicsHandleComponent|GrabComponentatLocation (Variables|Default|GetPhysicsHandle) _ragdoll_2 _returnvalue_2 _bonelocation)
        (else
          (Physics|Components|PhysicsHandle|ReleaseComponent (Variables|Default|GetPhysicsHandle)))))))

(fn Throw
  (params (Orientation :type Vector :default "0, 0, 0"))
  (Utilities|IsValid (Variables|Default|GetRagdoll)
    (:Is%20Valid
      (Physics|AddImpulse (Variables|Default|GetRagdoll) (* Orientation 5e+04) "spine_01" true))))

(fn Levitate
  (params (Destination :type Vector :default "0, 0, 0"))
  (bind _ragdoll (Variables|Default|GetRagdoll))
  (Utilities|IsValid (Variables|Default|GetRagdoll)
    (:Is%20Valid
      (Physics|Components|PhysicsHandle|SetTargetLocation (Variables|Default|GetPhysicsHandle) Destination)
      (bind _returnvalue (Physics|GetPhysicsLinearVelocity _ragdoll "spine_01"))
      (Physics|SetPhysicsLinearVelocity _ragdoll (* _returnvalue 0.5) false "spine_01"))))

(fn Attract
  (params (Destination :type Vector :default "0, 0, 0"))
  (Utilities|IsValid (Variables|Default|GetRagdoll)
    (:Is%20Valid
      (Physics|AddRadialForce (Variables|Default|GetRagdoll) Destination 1e+05 -5e+03 "RIF_Constant" true))))

(fn AssignRagdoll
  (params (Ragdoll :type Skeletal%20Mesh%20Component%20Object%20Reference))
  (bind _output_get (Variables|Default|SetRagdoll Ragdoll))
  (Transformation|AttachActorToActor (Components|GetOwner _output_get) self "None" "KeepWorld" "KeepWorld" "KeepWorld" false)
  (CallFunction|PrepareOutline))